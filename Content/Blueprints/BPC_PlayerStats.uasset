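; Actor component that tracks the player's current and maximum health in a top-down game.
; On BeginPlay it casts its owner to BP_TopDownCharacter and caches it to reach that character's HUD widget.
; Functions decrease health, raise max health, or add health capped at the maximum, each pushing the values to the health bar and text.
; DecreaseHealth also returns whether health has dropped to zero or below.
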(event `self.ReceiveBeginPlay`
  (bind _asbp_top_down_character (cast `/Game/TopDown/Blueprints/BP_TopDownCharacter` (`self.GetOwner`)))
  (set `self.Player Character BP` _asbp_top_down_character))

(fn `Decrease Health`
  (params (Damage :type "Float (double-precision)"))
  (returns (`Is Player Dead` :type Boolean))
  (bind _hud_widget (`/Game/TopDown/Blueprints/BP_TopDownCharacter.HUD Widget` (`self.Player Character BP`)))
  (bind _output_get (set `self.Current Health` (- (`self.Current Health`) Damage)))
  (`ProgressBar.SetPercent` (`/Game/UI/WB_HUD.HealthBar` _hud_widget) (/ _output_get (`self.Max Health`)))
  (`TextBlock.SetText` (`/Game/UI/WB_HUD.HealthText` _hud_widget) (`KismetTextLibrary.Conv_DoubleToText` (`self.Current Health`) "HalfToEven"))
  (if (<= (`self.Current Health`) 0.0)
    (return true)
    (else
      (return false))))

(fn `Increase Health`
  (params (`Added Health` :type "Float (double-precision)"))
  (bind _hud_widget (`/Game/TopDown/Blueprints/BP_TopDownCharacter.HUD Widget` (`self.Player Character BP`)))
  (set `self.Current Health` (+ (`self.Current Health`) `Added Health`))
  (if (> (`self.Current Health`) (`self.Max Health`))
    (set `self.Current Health` (`self.Max Health`)))
  (`ProgressBar.SetPercent` (`/Game/UI/WB_HUD.HealthBar` _hud_widget) (/ (`self.Current Health`) (`self.Max Health`)))
  (`TextBlock.SetText` (`/Game/UI/WB_HUD.HealthText` _hud_widget) (`KismetTextLibrary.Conv_DoubleToText` (`self.Current Health`) "HalfToEven")))

(fn `Increase Max Health`
  (params (`Health Incrementation` :type "Float (double-precision)"))
  (bind _hud_widget (`/Game/TopDown/Blueprints/BP_TopDownCharacter.HUD Widget` (`self.Player Character BP`)))
  (set `self.Max Health` (+ (`self.Max Health`) `Health Incrementation`))
  (`ProgressBar.SetPercent` (`/Game/UI/WB_HUD.HealthBar` _hud_widget) (/ (`self.Current Health`) (`self.Max Health`)))
  (`TextBlock.SetText` (`/Game/UI/WB_HUD.HealthText` _hud_widget) (`KismetTextLibrary.Conv_DoubleToText` (`self.Current Health`) "HalfToEven")))